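; Manager actor that gathers every PointLight in the level on BeginPlay and can make one breathe by animating its intensity.
; StartBreatheLight stores the first light's intensity, then plays a Timeline at a random rate, scaling that intensity by the curve.
; Only the first light in the array is affected; a loop over all lights exists but is never executed.
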(event Custom|StartBreatheLight
  (bind _pointlight (Variables|Default|GetpointLight))
  (bind _output (Utilities|Array|Get(acopy) _pointlight))
  (bind _pointlightcomponent (Variables|/Script/Engine.PointLight|GetPointLightComponent _output))
  (Variables|Default|SetOgIntensity (Variables|/Script/Engine.LightComponentBase|GetIntensity _pointlightcomponent))
  (Components|Timeline|SetPlayRate (Variables|Default|GetTimeline) (/ 1.0 (Math|Random|RandomFloatinRange 1.0 6.2)))
  (bind _newtrack_0 (Timeline|Timeline Play)
    (:Update
      (Rendering|Components|Light|SetIntensity _pointlightcomponent (* (Variables|Default|GetOgIntensity) _newtrack_0)))))

(event EventBeginPlay
  (bind _outactors (Actor|GetAllActorsOfClass "/Script/Engine.PointLight"))
  (Variables|Default|SetpointLight _outactors))

(event EventTick
  (params (DeltaSeconds :type Float%20%28single-precision%29)))

(fn ConstructionScript)