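; Credits manager actor that plays a timed title and subtitle intro in VR, locking player movement until the sequence ends.
; ExecuteSequence chains delays with FadeOutBlack, which plays or reverses a timeline on BlackWidget's opacity according to its alpha, and ChangeText, which toggles both text widgets' visibility.
; FadeSubtitle finally drives the subtitle's opacity and the alpha of a dynamic black material on an enclosing sphere from one timeline.
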(event Custom|ShowTitle
  (Rendering|SetVisibility (Variables|Default|GetTitleWidget) true false)
  (Rendering|SetVisibility (Variables|Default|GetSubtitleWidget) false false))

(event Custom|FadeOutBlack
  (if (<= (Variables|Default|GetAlpha) 0.0)
    (bind _out (Timeline|FadeOut ReverseFromEnd)
      (:Update
        (Class|WidgetComponent|SetTintColorandOpacity (Variables|Default|GetBlackWidget) (Math|Color|MakeColor 0.0 0.0 0.0 _out))
        (Variables|Default|SetAlpha (.A (Math|Color|BreakColor (Math|Color|MakeColor 0.0 0.0 0.0 _out))))))
    (else
      (Timeline|FadeOut PlayFromStart))))

(event Custom|HideBoth
  (Rendering|SetVisibility (Variables|Default|GetSubtitleWidget) false false)
  (Rendering|SetVisibility (Variables|Default|GetTitleWidget) false false))

(event Custom|ChangeText
  (bind _subtitlewidget (Variables|Default|GetSubtitleWidget))
  (bind _titlewidget (Variables|Default|GetTitleWidget))
  (Rendering|SetVisibility _subtitlewidget (not (Class|WidgetComponent|IsWidgetVisible _subtitlewidget)) false)
  (Rendering|SetVisibility _titlewidget (not (Class|WidgetComponent|IsWidgetVisible _titlewidget)) false))

(event Custom|ExecuteSequence
  (bind _asvr_player_pawn (Utilities|Casting|CastToVR_Player_Pawn (Game|Player|GetPlayerPawn 0)))
  (Variables|/Game/Pedro/Player/VR_Player_Pawn.VR_Player_Pawn_C|Setcan_move _asvr_player_pawn false)
  (Rendering|Material|SetScalarParameterValue (Variables|Default|Getblack_sphere) "alpha" 1.0 :!class /Script/Engine.MaterialInstanceDynamic)
  (Utilities|FlowControl|Delay 7.0)
  (CallFunction|FadeOutBlack)
  (Utilities|FlowControl|Delay 5.0)
  (CallFunction|FadeOutBlack)
  (Utilities|FlowControl|Delay 1.2)
  (CallFunction|ChangeText)
  (CallFunction|FadeOutBlack)
  (Utilities|FlowControl|Delay 5.0)
  (CallFunction|FadeSubtitle)
  (Variables|/Game/Pedro/Player/VR_Player_Pawn.VR_Player_Pawn_C|Setcan_move _asvr_player_pawn true))

(event Custom|FadeSubtitle
  (bind _out (Timeline|Timeline PlayFromStart)
    (:Update
      (Class|WidgetComponent|SetTintColorandOpacity (Variables|Default|GetSubtitleWidget) (Math|Color|MakeColor 0.0 0.0 0.0 _out))
      (Rendering|Material|SetScalarParameterValue (Variables|Default|Getblack_sphere) "alpha" _out :!class /Script/Engine.MaterialInstanceDynamic))))

(event Collision|EventActorBeginOverlap
  (params (OtherActor :type Actor%20Object%20Reference)))

(event EventTick
  (params (DeltaSeconds :type Float%20%28single-precision%29)))

(event EventBeginPlay
  (Rendering|SetVisibility (Variables|Default|GetBlackWidget) true false)
  (bind _returnvalue (Rendering|Material|CreateDynamicMaterialInstance (Variables|Default|Getinside_sphere) 0 "/Game/Pedro/Menu/Title/black.black" "None" :!class /Script/Engine.PrimitiveComponent))
  (Variables|Default|Setblack_sphere _returnvalue))

(fn ConstructionScript)