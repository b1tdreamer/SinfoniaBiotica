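; GSAnimator_BP drives a Niagara reveal and dissipate animation, synced with FMOD controller cues.
; At BeginPlay it writes its location to the GSVFXAnim_NPC parameter collection and caches FMOD_Main_Controller and GameManager.
; The AlphaAnim timeline, scaled to RevealAnimLEngth, feeds AnimProgress forward or reversed and calls AnimationEnd on GameManager when finished.
; RevealAnim delays its intro audio call; DissipateAnimation calls the disappearance cue immediately; RevealAnimNoMusic skips audio.
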(event Custom|RevealAnim
  (params (level :type Integer))
  (Utilities|FlowControl|Sequence
    (:then_0
      (Components|Timeline|SetPlayRate (Variables|Default|GetAlphaAnim) (/ 1.0 (Variables|Default|GetRevealAnimLEngth)))
      (bind _alpha (Timeline|AlphaAnim PlayFromStart)
        (:Update
          (bind _returnvalue (Class|NiagaraFunctionLibrary|GetNiagaraParameterCollection "/Game/VFX/GSVFXAnim_NPC.GSVFXAnim_NPC"))
          (Effects|Components|ParticleSystem|SetFloatParameter _returnvalue "AnimProgress" _alpha))
        (:Finished
          (Default|AnimationEnd (Variables|Default|GetGM_actor)))))
    (:then_1
      (Utilities|FlowControl|Delay 3.5)
      (Development|PrintString (Utilities|String|ToString(Integer) level))
      (Default|IntroAnimationStart (Variables|Default|Getcmp_main_controlle) level))))

(event Custom|DissipateAnimation
  (params (level :type Integer))
  (Default|DissapearanceAnimationEnd (Variables|Default|Getcmp_main_controlle) level)
  (Components|Timeline|SetPlayRate (Variables|Default|GetAlphaAnim) (/ 1.0 (Variables|Default|GetRevealAnimLEngth)))
  (bind _alpha (Timeline|AlphaAnim ReverseFromEnd)
    (:Update
      (bind _returnvalue (Class|NiagaraFunctionLibrary|GetNiagaraParameterCollection "/Game/VFX/GSVFXAnim_NPC.GSVFXAnim_NPC"))
      (Effects|Components|ParticleSystem|SetFloatParameter _returnvalue "AnimProgress" _alpha))
    (:Finished
      (Default|AnimationEnd (Variables|Default|GetGM_actor)))))

(event Custom|RevealAnimNoMusic
  (Components|Timeline|SetPlayRate (Variables|Default|GetAlphaAnim) (/ 1.0 (Variables|Default|GetRevealAnimLEngth)))
  (bind _alpha (Timeline|AlphaAnim PlayFromStart)
    (:Update
      (bind _returnvalue (Class|NiagaraFunctionLibrary|GetNiagaraParameterCollection "/Game/VFX/GSVFXAnim_NPC.GSVFXAnim_NPC"))
      (Effects|Components|ParticleSystem|SetFloatParameter _returnvalue "AnimProgress" _alpha))
    (:Finished
      (Default|AnimationEnd (Variables|Default|GetGM_actor)))))

(event EventBeginPlay
  (bind _returnvalue (Class|NiagaraFunctionLibrary|GetNiagaraParameterCollection "/Game/VFX/GSVFXAnim_NPC.GSVFXAnim_NPC"))
  (Effects|Components|ParticleSystem|SetVectorParameter _returnvalue "StartPosWS" (Transformation|GetActorLocation))
  (bind _returnvalue_2 (Actor|GetActorOfClass "/Game/FMOD/FMOD_Main_Controller.FMOD_Main_Controller_C"))
  (Variables|Default|Setcmp_main_controlle _returnvalue_2)
  (bind _returnvalue_3 (Actor|GetActorOfClass "/Game/Manager/GameManager.GameManager_C"))
  (Variables|Default|SetGM_actor _returnvalue_3))

(event Collision|EventActorBeginOverlap
  (params (OtherActor :type Actor%20Object%20Reference)))

(event EventTick
  (params (DeltaSeconds :type Float%20%28single-precision%29)))

(fn ConstructionScript)